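; Blueprint function library with helpers that safely read user data fields from JSON objects.
; GetUserObject returns a nested object field and GetUserValue returns a string field, each only after a HasField check.
; GetUserObjectValue chains the two to read a string one level down inside a named child object.
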(fn GetUserObjectValue
  (params (Json%20Obj :type Play%20Fab%20Json%20Object%20Object%20Reference) (To%20Find :type String) (To%20Find%20Value :type String))
  (return (CallFunction|GetUserValue (CallFunction|GetUserObject Json%20Obj To%20Find) To%20Find%20Value)))

(fn GetUserObject
  (params (Json%20Obj :type Play%20Fab%20Json%20Object%20Object%20Reference) (To%20Find :type String))
  (if (Class|PlayFabJsonObject|HasField Json%20Obj To%20Find)
    (return (Class|PlayFabJsonObject|GetObjectField Json%20Obj To%20Find))))

(fn GetUserValue
  (params (Json%20Obj :type Play%20Fab%20Json%20Object%20Object%20Reference) (ToFind :type String))
  (if (Class|PlayFabJsonObject|HasField Json%20Obj ToFind)
    (return (Class|PlayFabJsonObject|GetStringField Json%20Obj ToFind))))