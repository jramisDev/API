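; GameInstance Blueprint that handles PlayFab account login and holds the user's session data.
; LoginPlayFab sends username and password to PlayFab, printing the error on failure.
; On success it stores the PlayFab ID, session ticket and entity token, re-saves the existing credential variables, and calls LoginSuccessfuly.
; VerifyUserLogged logs in with stored credentials when the session ticket is empty, and a getter exposes the data.
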(event Custom|Login%20Success
  (params (result :type Client%20Login%20Result%20Structure) (customData :type Object%20Object%20Reference))
  (bind (_entitytoken _inforesultpayload _lastlogintime _newlycreated _playfabid _sessionticket) (Utilities|Struct|BreakClientLoginResult result))
  (CallFunction|SetUserLoginData (Variables|Default|GetUsuario) (Variables|Default|GetPassword) _playfabid _sessionticket _entitytoken)
  (Development|PrintString _playfabid)
  (Default|CallLoginSuccessfuly))

(event Custom|Login%20Failure
  (params (error :type Play%20Fab%20Error%20Structure) (customData :type Object%20Object%20Reference))
  (Development|PrintString (.ErrorMessage (Utilities|Struct|BreakPlayFabError error))))

(event Custom|LoginPlayFab
  (params (Username :type String) (Password :type String))
  (|LoginwithPlayFab (Utilities|Struct|MakeClientLoginWithPlayFabRequest 0 0 Password Username) (delegate Custom|Login%20Success) (delegate Custom|Login%20Failure)))

(fn SetUserLoginData
  (params (Usuario :type String) (Password :type String) (PlayFabId :type String) (SessionTick :type String) (EntityToken :type Play%20Fab%20Json%20Object%20Object%20Reference))
  (Variables|Default|SetUsuario Usuario)
  (Variables|Default|SetPassword Password)
  (Variables|Default|SetPlayFabId PlayFabId)
  (Variables|Default|SetSessionTick SessionTick)
  (Variables|Default|SetEntityToken EntityToken))

(fn GetUserLoginData
  (return (Variables|Default|GetUsuario) (Variables|Default|GetPassword) (Variables|Default|GetPlayFabId) (Variables|Default|GetSessionTick) (Variables|Default|GetEntityToken)))

(fn VerifyUserLogged
  (if (Utilities|Enum|NotEqual(Enum) (Variables|Default|GetSessionTick) "")
    (Development|PrintString "Logged")
    (else
      (CallFunction|LoginPlayFab (Variables|Default|GetUsuario) (Variables|Default|GetPassword)))))